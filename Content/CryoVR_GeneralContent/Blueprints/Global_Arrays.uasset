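; Global_Arrays is a Blueprint in CryoVR that tracks the current procedure step and logs the user's exam steps.
; MovetoNextStep advances Status only when it matches the expected current step.
; ExamRecordStep skips repeats of the last logged step, otherwise appending the step, its IndexDescriptions text and a timestamp to three parallel arrays.
; RecordCurrentStep and NewFunction_0 are empty stubs.
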(fn SetStatus
  (params (step :type Integer))
  (Variables|Default|SetStatus step))

(fn GetStatus
  (return (Variables|Default|GetStatus)))

(fn RecordCurrentStep
  (params (CurrentStep :type Integer)))

(fn MovetoNextStep
  (params (CurrentStep :type Integer) (NextStep :type Integer))
  (bind _step (CallFunction|GetStatus))
  (if (== _step CurrentStep)
    (CallFunction|SetStatus NextStep)))

(fn NewFunction0)

(fn ExamRecordStep
  (params (Step :type Integer))
  (bind _user_index_array (Variables|Exam|GetUser_Index_Array))
  (if (>= (Utilities|Array|Length _user_index_array) 1)
    (if (!= Step (Utilities|Array|Get(acopy) _user_index_array (- (Utilities|Array|Length _user_index_array) 1)))
      (Utilities|Array|Add (Variables|Exam|GetUser_Index_Array) Step :!label _label)
      (Utilities|Array|Add (Variables|Exam|GetUser_Description_Array) (.Value (Utilities|Map|Find (Variables|Exam|GetIndex&Descriptions) Step)))
      (Utilities|Array|Add (Variables|Exam|GetUser_Time_Array) (Utilities|Time|GetTimeSeconds)))
    (else
      (goto _label))))